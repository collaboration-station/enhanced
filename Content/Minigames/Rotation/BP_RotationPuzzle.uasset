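; BP_RotationPuzzle runs one round of the rotation minigame, from tile layout to completion and replacement.
; On begin play it positions the start and end tiles, lays out the tile grid between screen bounds and fades it in.
; Completion plays a sound, locks rotation, glows the end tile and awards points via MinigameGameMode.
; When the sound ends, the same timeline fades tiles out, then the puzzle spawns its successor and destroys itself with its tiles.
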(event OnAudioFinished(CompletionSound)
  ;[1 1 1] Fade out after the completion sound ends
  (bind (_direction _opacity) (Timeline|FadeOut PlayFromStart)
    (:Update
      (bind _tile (Utilities|ForEachTile)
        (:Body
          (bind _asbp_rotatable_tile (Utilities|Casting|CastToBP_RotatableTile _tile)
            (:then
              (Default|SetOpacity _asbp_rotatable_tile _opacity))
            (:CastFailed
              (Development|PrintString "Unexpected tile class"))))))
    (:Finished
      ;[1 1 1] When done fading out, spawn a new puzzle and destroy myself
      (switch Utilities|FlowControl|Switch|SwitchonETimelineDirection _direction
        (:Forward
          (Game|SpawnActorfromClass "BP_RotationPuzzle_C" (Transformation|GetActorTransform) "AlwaysSpawn" 0 0)
          (Actor|DestroyActor))))))

(event EventBeginPlay
  ;[1 1 1] Start all the tiles in the right positions
  (Utilities|CreateStartandEndTiles
    (:Done
      (bind (_tile _column _row) (Utilities|ForEachTile)
        (:Body
          (Transformation|SetActorLocation _tile (CallFunction|CalculateScreenPosition _column _row) false true)
          (bind _asbp_rotatable_tile (Utilities|Casting|CastToBP_RotatableTile _tile))
          (Default|SetOpacity _asbp_rotatable_tile 0.0))
        (:Done
          (bind (_direction _opacity) (Timeline|FadeOut ReverseFromEnd)
            (:Update
              (bind _tile_2 (Utilities|ForEachTile)
                (:Body
                  (bind _asbp_rotatable_tile_2 (Utilities|Casting|CastToBP_RotatableTile _tile_2)
                    (:then
                      (Default|SetOpacity _asbp_rotatable_tile_2 _opacity))
                    (:CastFailed
                      (Development|PrintString "Unexpected tile class"))))))
            (:Finished
              ;[1 1 1] When done fading out, spawn a new puzzle and destroy myself
              (switch Utilities|FlowControl|Switch|SwitchonETimelineDirection _direction
                (:Forward
                  (Game|SpawnActorfromClass "BP_RotationPuzzle_C" (Transformation|GetActorTransform) "AlwaysSpawn" 0 0)
                  (Actor|DestroyActor))))))))))

(event EventOnPuzzleComplete
  ;[1 1 1] Handle puzzle completion
  (Audio|Components|Audio|Play (Variables|Default|GetCompletionSound) 0.0)
  (Variables|Default|SetCanRotateTile false)
  (bind _asbp_image_tile (Utilities|Casting|CastToBP_ImageTile (Variables|/Script/Engine.ChildActorComponent|GetChildActor (Variables|Default|GetEndTile)))
    (:then
      (Default|Glow _asbp_image_tile)
      (bind _asminigame_game_mode (Utilities|Casting|CastToMinigameGameMode (Game|GetGameMode)))
      (Class|MinigameGameMode|AddPoints _asminigame_game_mode (Variables|Default|GetPointsPerPuzzle)))
    (:CastFailed
      (Development|PrintString "Unexpected tile class"))))

(event EventDestroyed
  ;[1 1 1] Destroy my tiles when I am destroyed.
  (bind _tile (Utilities|ForEachTile)
    (:Body
      (Actor|DestroyActor _tile))))

(fn ConstructionScript)

(fn CalculateScreenPosition
  (params (Column :type Integer) (Row :type Integer))
  (return (Math|Vector|MakeVector (Math|Float|Lerp (Variables|PuzzleConfiguration|GetPuzzleLeft) (Variables|PuzzleConfiguration|GetPuzzleRight) (/ (Math|Conversions|ToFloat(Integer) Column) (Math|Conversions|ToFloat(Integer) (Variables|Default|GetMaxColumns)))) (Math|Float|Lerp (Variables|PuzzleConfiguration|GetPuzzleTop) (Variables|PuzzleConfiguration|GetPuzzleBottom) (/ (Math|Conversions|ToFloat(Integer) Row) (Math|Conversions|ToFloat(Integer) (Variables|Default|GetMaxRows)))) 0.0)))