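; A touch-rotatable pipe tile (L, I or T shape) for the rotation puzzle minigame.
; BeginPlay builds a dynamic material for its pipe type, applies its orientation and caches the owning BP_RotationPuzzle.
; A touch plays a timeline quarter-turn, locking the puzzle's shared CanRotateTile flag, and calls Turn to update the model layer only when it finishes.
; Glow changes and SetOpacity drive material parameters, with sounds for sliding, blocked and charged turns.
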(event OnInputTouchBegin(Plane)
  (params (FingerIndex :type ETouchIndex%20Enum :default "Touch1") (TouchedComponent :type Primitive%20Component%20Object%20Reference))
  (if (Variables|/Game/Minigames/Rotation/BP_RotationPuzzle.BP_RotationPuzzle_C|GetCanRotateTile (Variables|Default|GetPuzzleBlueprintObject))
    (Audio|PlaySound2D "/Game/Minigames/SlidingTile/A_TileSlide.A_TileSlide")
    (Variables|/Game/Minigames/Rotation/BP_RotationPuzzle.BP_RotationPuzzle_C|SetCanRotateTile (Variables|Default|GetPuzzleBlueprintObject) false)
    (Variables|Default|SetInitialRotation (.yaw (Transformation|GetActorRotation)))
    (bind _rotationpercent (Timeline|TileRotation PlayFromStart)
      (:Update
        (Transformation|SetActorRelativeRotation (Math|Rotator|MakeRotator 0.0 0.0 (+ (Variables|Default|GetInitialRotation) (* _rotationpercent 9e+01)))))
      (:Finished
        (Transformation|SetActorRotation (Math|Rotator|MakeRotator 0.0 0.0 (+ (Variables|Default|GetInitialRotation) 9e+01)))
        (Variables|/Game/Minigames/Rotation/BP_RotationPuzzle.BP_RotationPuzzle_C|SetCanRotateTile (Variables|Default|GetPuzzleBlueprintObject) true)
        (Class|RotatableTile|Turn) ; Apply transformation to the model layer at the end of the animation.
        (if (Variables|Default|GetbGlowing)
          (Audio|PlaySound2D "/Game/Minigames/Rotation/A_RotationCharged.A_RotationCharged"))))
    (else
      (Audio|PlaySound2D "/Game/Minigames/SlidingTile/A_CannotMove.A_CannotMove"))))

(event EventBeginPlay
  ;[1 1 1] Initialize the tile
  (bind _returnvalue (Rendering|Material|CreateDynamicMaterialInstance (Variables|Default|GetPlane) 0 "/Game/Minigames/Rotation/M_Pipe.M_Pipe" :!class /Script/Engine.PrimitiveComponent))
  (bind _output_get (Variables|Default|SetDynamicMaterial _returnvalue))
  (Rendering|Material|SetTextureParameterValue _output_get "Texture" (Utilities|Select :Index (Variables|Default|GetType) :Type_L "/Game/Minigames/Rotation/T_Pipe_L.T_Pipe_L" :Type_I "/Game/Minigames/Rotation/T_Pipe_I.T_Pipe_I" :Type_T "/Game/Minigames/Rotation/T_Pipe_T.T_Pipe_T"))
  (Rendering|Material|SetMaterial (Variables|Default|GetPlane) 0 _returnvalue)
  (Transformation|SetActorRotation (Math|Rotator|MakeRotator 0.0 0.0 (Variables|Default|GetOrientation)))
  (bind _asbp_rotation_puzzle (Utilities|Casting|CastToBP_RotationPuzzle (Variables|Default|GetPuzzle))
    (:then
      (Variables|Default|SetPuzzleBlueprintObject _asbp_rotation_puzzle))
    (:CastFailed
      (Development|PrintString "Unexpected puzzle type"))))

(event EventOnGlowChange
  (params (Glowing :type Boolean))
  ;[1 1 1] Update glow texture parameter on glow change
  (bind _asmaterial_instance_dynamic (Utilities|Casting|CastToMaterialInstanceDynamic (Rendering|Material|GetMaterial (Variables|Default|GetPlane) 0)))
  (Rendering|Material|SetScalarParameterValue _asmaterial_instance_dynamic "Glow" (select Glowing 1.0 0.0) :!class /Script/Engine.MaterialInstanceDynamic))

(fn ConstructionScript)

(fn SetOpacity
  (params (Opacity :type Float%20%28single-precision%29))
  (Rendering|Material|SetScalarParameterValue (Variables|Default|GetDynamicMaterial) "Opacity" Opacity :!class /Script/Engine.MaterialInstanceDynamic))