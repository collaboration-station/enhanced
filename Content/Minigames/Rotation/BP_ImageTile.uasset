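; BP_ImageTile is a tile actor for the rotation minigame that shows either a circuit start or circuit end image.
; On BeginPlay it creates a dynamic instance of M_Pipe, picks the texture from the Start flag and applies the material to its static mesh.
; A Glow function sets the material's Glow parameter to light the tile up, with no logic here to turn it back off.
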(event EventBeginPlay
  (bind _returnvalue (Rendering|Material|CreateDynamicMaterialInstance "/Game/Minigames/Rotation/M_Pipe.M_Pipe" :!class /Script/Engine.KismetMaterialLibrary))
  (bind _output_get (Variables|Default|SetDynamicMaterial _returnvalue))
  (Rendering|Material|SetTextureParameterValue _output_get "Texture" (select (Variables|Default|GetStart) "/Game/Minigames/Rotation/T_CircuitStart.T_CircuitStart" "/Game/Minigames/Rotation/T_CircuitEnd.T_CircuitEnd"))
  (Rendering|Material|SetMaterial (Variables|Default|GetStaticMesh) 0 (Variables|Default|GetDynamicMaterial)))

(event Collision|EventActorBeginOverlap
  (params (OtherActor :type Actor%20Object%20Reference)))

(event EventTick
  (params (DeltaSeconds :type Float%20%28single-precision%29)))

(fn ConstructionScript)

(fn Glow
  (Rendering|Material|SetScalarParameterValue (Variables|Default|GetDynamicMaterial) "Glow" 1.0 :!class /Script/Engine.MaterialInstanceDynamic))