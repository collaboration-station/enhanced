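; Touchable button actor for a Simon-style sequence minigame that lights up and plays its sound.
; The construction script creates a dynamic material on the sphere tinted with the button's color.
; Play swaps to the active sprite, raises the material's active parameter and plays audio, then reverts after a delay.
; Touch input forwards the button to its Puzzle via OnButtonTouched, leaving sequence logic there.
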(event Custom|Play
  (Rendering|Material|SetScalarParameterValue (Variables|Default|GetBackgroundMaterial) (Variables|Constants|GetMaterialActiveParameter) 1.0 :!class /Script/Engine.MaterialInstanceDynamic)
  (Audio|Components|Audio|Play (Variables|Default|GetAudio) 0.0)
  (Rendering|Components|Sprite|SetSprite (Variables|Default|GetSprite) (Variables|Default|GetActiveSprite))
  (Utilities|FlowControl|Delay (Variables|Constants|GetDelayBetweenFrames))
  (Rendering|Components|Sprite|SetSprite (Variables|Default|GetSprite) (Variables|Default|GetInactiveSprite))
  (Rendering|Material|SetScalarParameterValue (Variables|Default|GetBackgroundMaterial) (Variables|Constants|GetMaterialActiveParameter) 0.0 :!class /Script/Engine.MaterialInstanceDynamic))

(event EventBeginPlay
  (Rendering|Components|Sprite|SetSprite (Variables|Default|GetSprite) (Variables|Default|GetInactiveSprite))
  (Audio|Components|Audio|SetSound (Variables|Default|GetAudio) (Variables|Default|GetSound)))

(event EventActorOnInputTouchBegin
  (params (FingerIndex :type ETouchIndex%20Enum :default "Touch1"))
  (Default|OnButtonTouched (Variables|Default|GetPuzzle) self))

(fn ConstructionScript
  (bind _returnvalue (Rendering|Material|CreateDynamicMaterialInstance (Variables|Default|GetSphere) 0 "/Game/Minigames/Simon/M_SequenceButtonBackground.M_SequenceButtonBackground" :!class /Script/Engine.PrimitiveComponent))
  (bind _output_get (Variables|Default|SetBackgroundMaterial _returnvalue))
  (Rendering|Material|SetVectorParameterValue _output_get "Color" (Variables|Default|GetColor) :!class /Script/Engine.MaterialInstanceDynamic))