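; Game mode for the sliding tile minigame that runs an endless series of puzzles of rising difficulty.
; On BeginPlay it spawns a BP_SlidingTilePuzzle with the current shuffle count and a randomly chosen picture material.
; On completion it awards points, destroys the puzzle, increments the shuffles and spawns the next.
; It also holds helper functions, not called here, that map tile indices to offset grid positions on the XZ plane.
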(event Custom|OnPuzzleComplete
  (Class|MinigameGameMode|AddPoints (Variables|Default|GetPointsPerPuzzle))
  (Actor|DestroyActor (stale _returnvalue))
  (Math|Integer|IncrementInt (Variables|Default|GetStartingShuffles)
    (:%20%20
      (bind _returnvalue (Game|SpawnActorfromClass "/Game/Minigames/SlidingTile/BP_SlidingTilePuzzle.BP_SlidingTilePuzzle_C" (Math|Transform|MakeTransform (Variables|Constants|GetSpawnTransformLocation) "0, 0, 0" "1,1,1") "Undefined" 0 (Variables|Default|GetStartingShuffles) (Utilities|Select :Index (Math|Random|RandomIntegerinRange 0 3) :Option%200 "/Game/Minigames/SlidingTile/MI_Arrows.MI_Arrows" :Option%201 "/Game/Minigames/SlidingTile/MI_Peacock.MI_Peacock" :Option%202 "/Game/Minigames/SlidingTile/MI_Toucan.MI_Toucan" :Option%203 "/Game/Minigames/SlidingTile/MI_Cross.MI_Cross") 0))
      (EventDispatchers|BindEventtoOnPuzzleComplete _returnvalue (delegate Custom|OnPuzzleComplete)))))

(event EventBeginPlay
  (bind _returnvalue (Game|SpawnActorfromClass "/Game/Minigames/SlidingTile/BP_SlidingTilePuzzle.BP_SlidingTilePuzzle_C" (Math|Transform|MakeTransform (Variables|Constants|GetSpawnTransformLocation) "0, 0, 0" "1,1,1") "Undefined" 0 (Variables|Default|GetStartingShuffles) (Utilities|Select :Index (Math|Random|RandomIntegerinRange 0 3) :Option%200 "/Game/Minigames/SlidingTile/MI_Arrows.MI_Arrows" :Option%201 "/Game/Minigames/SlidingTile/MI_Peacock.MI_Peacock" :Option%202 "/Game/Minigames/SlidingTile/MI_Toucan.MI_Toucan" :Option%203 "/Game/Minigames/SlidingTile/MI_Cross.MI_Cross") 0))
  (EventDispatchers|BindEventtoOnPuzzleComplete _returnvalue (delegate Custom|OnPuzzleComplete)))

(fn ConstructionScript)

(fn DetermineTileLocation
  (params (index :type Integer))
  (return (- (Math|Vector|MakeVector (* (Math|Integer|%(Integer) index (Variables|Default|GetColumns)) (+ (Variables|Default|GetCellWidth) (Variables|Default|GetPaddingBetweenCells))) 0.0 (* (* (/ index (Variables|Default|GetRows)) (+ (Variables|Default|GetCellHeight) (Variables|Default|GetPaddingBetweenCells))) -1.0)) (CallFunction|MakeOffsetVector))))

(fn MakeOffsetVector
  (return (Math|Vector|MakeVector (* (+ (Variables|Default|GetCellWidth) (Variables|Default|GetPaddingBetweenCells)) (Math|Conversions|ToFloat(Integer) (/ (Variables|Default|GetColumns) 2))) 0.0 (* (* (+ (Variables|Default|GetCellHeight) (Variables|Default|GetPaddingBetweenCells)) (Math|Conversions|ToFloat(Integer) (/ (Variables|Default|GetRows) 2))) -1.0))))