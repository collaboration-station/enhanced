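; Sliding-tile puzzle minigame actor that lays out tiles, runs shuffle, play and completion phases, then signals completion.
; On BeginPlay a timeline spreads tile padding, the last tile moves off-screen as the gap, and a delayed macro loop shuffles by random legal moves.
; Each move animates via a timeline, faster or slower while shuffling.
; Solving restores the gap tile, reverses the padding and plays a sound before completion fires.
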(event EventBeginPlay
  ;[1 1 1] BeginPlay
  (bind (_direction _paddingsize) (Timeline|PaddingExtend Play)
    (:Update
      (Variables|Default|SetPaddingBetweenTiles _paddingsize)
      (CallFunction|UpdateAllTilePositions))
    (:Finished
      (if (Utilities|Enum|Equal(Enum) _direction "Forward")
        (CallFunction|RemoveLastTile)
        (Utilities|Shuffle
          (:Done
            (Variables|Default|SetState "NewEnumerator1")))
        (else
          (Audio|Components|Audio|Play (Variables|Default|GetCompletionSound) 0.0)
          (Variables|Default|SetState "NewEnumerator3"))))))

(event EventTick
  (params (DeltaSeconds :type Float%20%28single-precision%29))
  ;[1 1 1] On Tick, check if the puzzle completion sound has played and is over
  (if (and (Utilities|Enum|Equal(Enum) (Variables|Default|GetState) "NewEnumerator3") (not (Audio|Components|Audio|IsPlaying (Variables|Default|GetCompletionSound))))
    (Default|CallOnPuzzleComplete)))

(event EventDestroyed
  ;[1 1 1] Destroy all tiles when this puzzle is destroyed
  (for _array_element (Variables|Default|GetTiles)
    (Actor|DestroyActor _array_element)))

(event EventOnTileMoved
  (params (Tile :type Sliding%20Tile%20Object%20Reference) (From :type Int%20Point%20Structure) (To :type Int%20Point%20Structure))
  ;[1 1 1] On Tile Moved
  (Variables|Default|SetSlideAnimationPlaying true)
  (Components|Timeline|SetPlayRate (Variables|Default|GetSlideTile) (select (Utilities|Enum|Equal(Enum) (Variables|Default|GetState) "NewEnumerator0") (/ 1.0 (Variables|Default|GetSingleTileShuffleAnimationDuration)) 1.0))
  (bind _locationalpha (Timeline|SlideTile PlayFromStart)
    (:Update
      (Transformation|SetActorLocation Tile (Math|Vector|Lerp(Vector) (CallFunction|ComputeScreenPosition From) (CallFunction|ComputeScreenPosition To) _locationalpha) false false))
    (:Finished
      (Variables|Default|SetSlideAnimationPlaying false)
      (if (Class|SlidingTilePuzzle|IsSolved)
        (CallFunction|BringBackGapTile)
        (Components|Timeline|ReversefromEnd (Variables|Default|GetPaddingExtend))))))

(fn ConstructionScript)

(fn ComputeScreenPosition
  (params (PuzzlePosition :type Int%20Point%20Structure))
  (return (+ (- (Math|Vector|MakeVector (* (.x PuzzlePosition) (CallFunction|PaddedTileWidth)) 0.0 (* (* (.y PuzzlePosition) (CallFunction|PaddedTileHeight)) -1.0)) (Math|Vector|MakeVector (* (CallFunction|PaddedTileWidth) 2.0) 0.0 (+ (* (CallFunction|PaddedTileHeight) -2.0) 1.5e+02))) (Transformation|GetActorLocation))))

(fn PaddedTileWidth
  (return (+ (Variables|Default|GetTileWidth) (Variables|Default|GetPaddingBetweenTiles))))

(fn PaddedTileHeight
  (return (+ (Variables|Default|GetTileHeight) (Variables|Default|GetPaddingBetweenTiles))))

(fn IsTouchSlideEnabled
  (return (and (Utilities|Enum|Equal(Enum) (Variables|Default|GetState) "NewEnumerator1") (not (Variables|Default|GetSlideAnimationPlaying)))))

(fn UpdateAllTilePositions
  (for _array_element (Variables|Default|GetTiles)
    (Transformation|SetActorLocation _array_element (CallFunction|ComputeScreenPosition (Variables|/Script/CollaborationStation.SlidingTile|GetPosition _array_element)) false true)))

(fn RemoveLastTile
  (bind _tiles (Variables|Default|GetTiles))
  (bind _asbp_sliding_tile (Utilities|Casting|CastToBP_SlidingTile (Utilities|Array|Get(acopy) _tiles (- (Utilities|Array|Length _tiles) 1))))
  (bind _output_get (Variables|Default|SetRemovedTile _asbp_sliding_tile))
  (Transformation|SetActorLocation _output_get "10000.000000,10000.000000,10000.000000" false true) ; Move actor way off-screen
  (Class|SlidingTilePuzzle|RemoveTiletoCreateGap _output_get))

(fn BringBackGapTile
  (bind _removedtile (Variables|Default|GetRemovedTile))
  (Class|SlidingTilePuzzle|ReinsertGapTile _removedtile)
  (Transformation|SetActorLocation _removedtile (CallFunction|ComputeScreenPosition (Variables|/Script/CollaborationStation.SlidingTile|GetPosition _removedtile)) false false))