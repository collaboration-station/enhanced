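; BP_SlidingTile is a single touch-controlled tile in the sliding tile puzzle minigame.
; On BeginPlay it applies its material to its plane mesh and caches its Puzzle reference as a BP_SlidingTilePuzzle, printing an error on any other type.
; A touch on the plane asks the puzzle to move the tile if touch sliding is enabled and the move is allowed, otherwise it plays a cannot-move sound.
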(event OnInputTouchBegin(Plane)
  (params (FingerIndex :type ETouchIndex%20Enum :default "Touch1") (TouchedComponent :type Primitive%20Component%20Object%20Reference))
  (if (and (Default|IsTouchSlideEnabled (Variables|Default|GetPuzzleBlueprint)) (Class|SlidingTilePuzzle|CanMove (Variables|Default|GetPuzzle) self))
    (Class|SlidingTilePuzzle|Move (Variables|Default|GetPuzzle) self)
    (else
      (Audio|PlaySound2D "/Game/Minigames/SlidingTile/A_CannotMove.A_CannotMove"))))

(event EventBeginPlay
  (Rendering|Material|SetMaterial (Variables|Default|GetPlane) 0 (Variables|Default|GetMaterial))
  (bind _asbp_sliding_tile_puzzle (Utilities|Casting|CastToBP_SlidingTilePuzzle (Variables|Default|GetPuzzle))
    (:then
      (Variables|Default|SetPuzzleBlueprint _asbp_sliding_tile_puzzle))
    (:CastFailed
      (Development|PrintString "Unexpected puzzle type!"))))

(fn ConstructionScript)