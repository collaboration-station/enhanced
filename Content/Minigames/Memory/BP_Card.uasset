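; BP_Card is a card actor for the Memory minigame that handles its entry, flip and matched animations.
; On BeginPlay a timeline slides it from world origin to its placed location.
; PlayFlipEffect alternates the flip timeline forward and reverse, rotating yaw, swapping front/back material at halfway and signalling completion through OnFlipEffectComplete.
; PlayMatchedEffect starts a timer that calls FlyAway, lerping the card outward to FlyawayY.
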(event Custom|DoFlyAway
  (bind _returnvalue (Transformation|GetActorLocation))
  (bind _flyawaymultiplier (Variables|Flyaway|GetFlyAwayMultiplier))
  (bind _returnvalue_2 (* _returnvalue _flyawaymultiplier))
  ;[1 1 1] Fly Away after match
  (Utilities|Time|ClearandInvalidateTimerbyHandle (stale EventPlayMatchedEffect _returnvalue))
  (bind _output_get (Variables|EntryAnimation|SetDesiredLocation (Math|Vector|MakeVector (.x _returnvalue_2) (Variables|Flyaway|GetFlyawayY) (.z _returnvalue_2))))
  (bind _output_get_2 (Variables|Flyaway|SetStartLocation (Transformation|GetActorLocation)))
  (bind _percent (Timeline|FlyAwayTimeline PlayFromStart)
    (:Update
      (Transformation|SetActorLocation (Math|Vector|Lerp(Vector) _output_get_2 _output_get _percent) false false))))

(event EventBeginPlay
  ;[1 1 1] Animate card entry
  (Variables|EntryAnimation|SetDesiredLocation (Transformation|GetActorLocation))
  (Transformation|SetActorLocation "0, 0, 0" false false)
  (bind _percentcomplete (Timeline|AnimateToStartLocation PlayFromStart)
    (:Update
      (Transformation|SetActorLocation (Math|Vector|Lerp(Vector) "0, 0, 0" (Variables|EntryAnimation|GetDesiredLocation) _percentcomplete) false false)
      ;[1 1 1] Initialize flip timeline with desired duration
      (Components|Timeline|SetPlayRate (Variables|Default|GetFlipTimeline) (/ 1.0 (Variables|Flip|GetFlipDuration))))))

(event EventPlayMatchedEffect
  ;[1 1 1] Fly Away after match
  (bind _returnvalue (Utilities|Time|SetTimerbyFunctionName 0 "FlyAway" (Variables|Flyaway|GetDelayBeforeFlyaway))))

(event EventPlayFlipEffect
  (bind _cube (Variables|Default|GetCube))
  ;[1 1 1] Flip Effect
  (Audio|PlaySound2D "/Game/Minigames/Memory/Sound/S_CardFlip_Mono.S_CardFlip_Mono")
  (bind _isa (Utilities|FlowControl|FlipFlop)
    (:A
      (bind _rotation_percent (Timeline|FlipTimeline PlayFromStart)
        (:Update
          (Transformation|SetActorRotation (Math|Rotator|MakeRotator 0.0 0.0 (Math|Float|Lerp 0.0 1.8e+02 _rotation_percent))))
        (:Finished
          (Class|Card|OnFlipEffectComplete))
        (:Halfway
          (if _isa
            (Rendering|Material|SetMaterial _cube 0 (Variables|Default|GetCardFront))
            (else
              (Rendering|Material|SetMaterial _cube 0 (Variables|Default|GetCardBack)))))))
    (:B
      (Timeline|FlipTimeline ReverseFromEnd))))

(fn ConstructionScript)

(fn FlyAway
  (CallFunction|DoFlyAway))