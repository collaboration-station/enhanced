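; Card grid actor for the Memory minigame, handling mismatch feedback and replacement of a completed grid.
; On a mismatch it plays a failure sound and a timeline that randomly jitters both cards, then restores their positions and signals completion.
; On completion a short timer lets the last match finish, then the grid spawns its successor in place and destroys itself.
; The successor copies size and shuffle settings from its CloneSource on BeginPlay.
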(event Custom|OnDelayComplete
  ;[1 1 1] Pause while the last match flies away, then make a new grid
  (Utilities|Time|ClearandInvalidateTimerbyHandle (stale EventPlayGridCompleteEffect _returnvalue))
  (Game|SpawnActorfromClass "BP_Grid_C" (Transformation|GetActorTransform) "Undefined" 0 self 0)
  (Actor|DestroyActor))

(event EventPlayMismatchEffect
  (params (Card1 :type Card%20Object%20Reference) (Card2 :type Card%20Object%20Reference))
  (bind _returnvalue (Math|Random|RandomFloatinRange -1.0 1.0))
  ;[1 1 1] Play mismatch effect
  (Audio|Components|Audio|Play (Variables|Default|GetFailureSound) 0.0)
  (Variables|Default|SetMismatchCard1Location (Transformation|GetActorLocation Card1))
  (Variables|Default|SetMismatchCard2Location (Transformation|GetActorLocation Card2))
  (Timeline|MismatchEffect PlayFromStart
    (:Update
      (Transformation|AddActorLocalOffset Card1 (Math|Vector|MakeVector _returnvalue _returnvalue _returnvalue) false true)
      (Transformation|AddActorLocalOffset Card2 (Math|Vector|MakeVector _returnvalue _returnvalue _returnvalue) false false))
    (:Finished
      (Transformation|SetActorLocation Card1 (Variables|Default|GetMismatchCard1Location) false true)
      (Transformation|SetActorLocation Card2 (Variables|Default|GetMismatchCard2Location) false true)
      (Class|Grid|OnPlayMismatchEffectComplete))))

(event EventPlayGridCompleteEffect
  ;[1 1 1] Pause while the last match flies away, then make a new grid
  (bind _returnvalue (Utilities|Time|SetTimerbyFunctionName 0 "DelayComplete" 0.5)))

(event EventBeginPlay
  (bind _clonesource (Variables|Initialization|GetCloneSource)
    (:then
      (CallFunction|CopyAttributes _clonesource))
    (:else)))

(fn ConstructionScript)

(fn DelayComplete
  (CallFunction|OnDelayComplete))

(fn CopyAttributes
  (params (From :type BP%20Grid%20Object%20Reference))
  (Variables|Default|SetGridWidth (Variables|/Script/CollaborationStation.Grid|GetGridWidth From))
  (Variables|Default|SetGridHeight (Variables|/Script/CollaborationStation.Grid|GetGridHeight From))
  (Variables|Default|SetbShuffle (Variables|/Script/CollaborationStation.Grid|GetbShuffle From)))