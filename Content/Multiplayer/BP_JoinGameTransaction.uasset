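; Firebase-style database transaction that adds the logged-in user to a multiplayer game's player list.
; DoTransaction returns success without writing when the data is null, expecting a retry with real values.
; Otherwise it uses the current child count of "players" as the new slot key and writes the user's ID to that slot's "uid" field.
; Debug prints trace each step.
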(fn DoTransaction
  (params (MutableData :type Mutable%20Data%20Proxy%20Object%20Reference))
  (Development|PrintString 0 "In transaction")
  ;[1 1 1] If the value is null, just exit, since it will be called again with real values.
  (if (Class|DatabaseVariantProxy|IsNull (Class|MutableDataProxy|Value MutableData))
    (Development|PrintString 0 "Null value, try again")
    (return "TransactionResultSuccess")
    (else
      (Development|PrintString 0 "Not null, moving forward")
      (Utilities|FlowControl|Sequence
        (:then_0
          ;[1 1 1] Find the path to this player's location (e.g. players/1)
          (bind _output_get (Variables|Default|SetPlayer%20Path (Utilities|String|Append "players/" (Utilities|String|ToString(Integer) (Class|MutableDataProxy|ChildrenCount (Class|MutableDataProxy|Child MutableData "players"))))))
          (Development|PrintString 0 _output_get))
        (:then_1
          ;[1 1 1] Set the player uid
          (bind _returnvalue (Class|UltimateMobileKitAuth|GetLoggedUser))
          (Class|MutableDataProxy|SetValue (Class|MutableDataProxy|Child (Class|MutableDataProxy|Child MutableData (Variables|Default|GetPlayer%20Path)) "uid") (Class|DatabaseVariantProxy|ConstructfromString (.userid _returnvalue)))
          (Development|PrintString 0 "Set the UID for me"))
        (:then_2
          (return "TransactionResultSuccess"))))))