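; Firebase facade for multiplayer expeditions: creates or joins games by lobby code, with player 0 as commander.
; It writes state, minigame selections and scores to the database, relaying watched changes through dispatchers; joining and briefing use transactions.
; A game-instance memento restores it across level changes.
; Disconnecting or backgrounding flags an abort; cancelling only posts a 'cancelled' state because deletion crashes Android, leaving stale codes for recycling.
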(event ApplicationWillEnterBackgroundDelegate(ApplicationLifecycle)
  ;[1 1 1] Abort the game if the app goes into the background
  (if (Variables|Default|GetInGame)
    (bind _error (|DatabaseReferenceSetValue (Class|DatabaseReferenceProxy|Child (Variables|Default|GetGame%20Ref) "abort") (Class|DatabaseVariantProxy|ConstructfromBool true))
      (:OnSuccess
        (Variables|Default|SetInGame false))
      (:OnFailure
        (Utilities|LogError "Error marking game aborted due to backgrounding" _error)))))

(event Custom|ProceedToDebrief
  ;[1 1 1] Commander issues this command to proceed the game to debriefing
  (bind _error (|DatabaseReferenceSetValue (Class|DatabaseReferenceProxy|Child (Variables|Default|GetGame%20Ref) "state") (Class|DatabaseVariantProxy|ConstructfromString "debrief"))
    (:OnFailure
      (Utilities|LogError "Error setting game state to debrief" _error))))

(event Custom|Start%20Expedition
  ;[1 1 1] Start the expedition. This will assign country codes and get the game into the 'brief' state.
  (bind _error (|DatabaseReferenceRunTransaction (Variables|Default|GetGame%20Ref) "/Game/Multiplayer/BP_InitialBriefingTransaction.BP_InitialBriefingTransaction_C")
    (:OnFailure
      (Utilities|LogError "Problem with the initial briefing transaction" _error))))

(event Custom|Create%20Game
  ;[1 1 1] Create Game
  (Utilities|CreateGameandRegisterinLobby
    (:Done
      ;[1 1 1] Manage mission abort on disconnect
      (Utilities|ConfigureAbortMissiononDisconnect
        (:Done
          (Utilities|WatchforMissionAbort
            (:Done
              (Variables|Default|SetInGame true))))))))

(event Custom|AdvanceExpedition
  ;[1 1 1] Continue the expedition after completing a round
  (Utilities|ChangeGameState "brief"))

(event Custom|SelectMinigame
  (params (Minigame :type String) (Round :type Integer))
  ;[1 1 1] Select Minigame
  (bind _error (|DatabaseReferenceSetValue (Class|DatabaseReferenceProxy|Child (Variables|Default|GetGame%20Ref) (Utilities|String|Append "players/" (Utilities|String|ToString(Integer) (Variables|Default|GetPlayerIndex)) "/round-" (Utilities|String|ToString(Integer) Round) "/selection")) (Class|DatabaseVariantProxy|ConstructfromString Minigame))
    (:OnFailure
      (Utilities|LogError "Error setting minigame." _error))))

(event Custom|WatchMinigameSelections
  (params (Enable :type Boolean) (Round :type Integer))
  (bind _game_ref (Variables|Default|GetGame%20Ref))
  (bind _returnvalue (Class|DatabaseReferenceProxy|Child _game_ref "players"))
  ;[1 1 1] Watch for players to select their minigames for the given round
  (if Enable
    (bind _snapshot (|AddValueListener _returnvalue)
      (:OnValueChanged
        (bind _numberofplayerswithselections (CallFunction|CountPlayerswithMinigameSelection Round _snapshot))
        (Default|CallOnNumberOfMinigameSelectionsChanged _numberofplayerswithselections (== _numberofplayerswithselections (Variables|Default|GetNumber%20of%20Players)))))
    (else
      (Class|QueryProxy|RemoveValueListener _returnvalue))))

(event Custom|ComputeRoundScore
  ;[1 1 1] Compute the score (asynchronously) and respond via dispatcher
  (bind _score (Utilities|ComputeScoreforRound (Variables|Default|GetRoundNumber))
    (:Done
      (Default|CallOnScoreTotalComputed _score))))

(event Custom|StartRound
  ;[1 1 1] Start the round. Called by the commander once all the task selections are made.
  (bind _error (|DatabaseReferenceSetValue (Class|DatabaseReferenceProxy|Child (Variables|Default|GetGame%20Ref) "state") (Class|DatabaseVariantProxy|ConstructfromString "play"))
    (:OnFailure
      (Utilities|LogError "Error setting game state to play" _error))))

(event Custom|MarkRoundComplete
  (params (Score :type Integer))
  ;[1 1 1] Post this player's score to mark that they are done with their minigame.
  (bind _error (|DatabaseReferenceSetValue (Class|DatabaseReferenceProxy|Child (Variables|Default|GetGame%20Ref) (Utilities|String|Append "players/" (Utilities|String|ToString(Integer) (Variables|Default|GetPlayerIndex)) "/round-" (Utilities|String|ToString(Integer) (Variables|Default|GetRoundNumber)) "/score")) (Class|DatabaseVariantProxy|ConstructfromInteger Score))
    (:OnFailure
      (Utilities|LogError "Error posting this round's score" _error))))

(event Custom|Watch%20Game%20State
  (params (Enable :type Boolean))
  (bind _game_ref (Variables|Default|GetGame%20Ref))
  (bind _returnvalue (Class|DatabaseReferenceProxy|Child _game_ref "state"))
  ;[1 1 1] Enable watching the `state`, firing event dispatcher on change. Update country code when first going to 'brief' state.
  (if Enable
    (Utilities|FlowControl|DoOnce false :!label _label
      (:Completed
        (bind _snapshot (|AddValueListener _returnvalue)
          (:OnValueChanged
            (if (Utilities|Enum|Equal(Enum) (Class|DatabaseVariantProxy|StringValue (Class|DataSnapshotProxy|Value _snapshot)) "abort")
              (CallFunction|ShowAbortDialog)
              (else
                (if (CallFunction|IsTimetoSetCountryCode (Class|DatabaseVariantProxy|StringValue (Class|DataSnapshotProxy|Value _snapshot)))
                  (Utilities|ReadCountryCode
                    (:Done
                      (bind _count (Utilities|CountNumberOfPlayers)
                        (:Done
                          (Variables|Default|SetNumber%20of%20Players _count))))))
                (Default|CallGameStateChanged (Class|DatabaseVariantProxy|StringValue (Class|DataSnapshotProxy|Value _snapshot)))))))))
    (else
      (Class|QueryProxy|RemoveValueListener _returnvalue)
      (goto _label Reset))))

(event Custom|SaveToGameInstance
  ;[1 1 1] Save a memento of this object to the game instance
  (bind _asbp_collaboration_station_game_instance (Utilities|Casting|CastToBP_CollaborationStationGameInstance (Game|GetGameInstance)))
  (Variables|/Game/BP_CollaborationStationGameInstance.BP_CollaborationStationGameInstance_C|SetFacadeMemento _asbp_collaboration_station_game_instance (Utilities|Struct|MakeFFirebaseFacadeMemento (Variables|Default|GetPlayerIndex) (Variables|Default|GetRoundNumber) (Class|DatabaseReferenceProxy|Key (Variables|Default|GetGame%20Ref)) (Variables|Default|GetNumber%20of%20Players) (Variables|Default|GetIsCountryAssigned) (Variables|Default|GetCountry))))

(event Custom|WatchPlayerScores
  (params (Enable :type Boolean))
  (bind _game_ref (Variables|Default|GetGame%20Ref))
  (bind _returnvalue (Class|DatabaseReferenceProxy|Child _game_ref "players"))
  ;[1 1 1] Enable watching player scores
  (if Enable
    (bind _snapshot (|AddValueListener _returnvalue)
      (:OnValueChanged
        (bind _all (CallFunction|DoAllPlayersHaveScoresSet _snapshot))
        (if _all
          (Default|CallOnAllPlayersPostedScores))))
    (else
      (Class|QueryProxy|RemoveValueListener _returnvalue))))

(event Custom|MarkExpeditionComplete
  ;[1 1 1] Mark expedition as "done"
  (bind _error (|DatabaseReferenceSetValue (Class|DatabaseReferenceProxy|Child (Variables|Default|GetGame%20Ref) "state") (Class|DatabaseVariantProxy|ConstructfromString "done"))
    (:OnSuccess
      (Variables|Default|SetInGame false))
    (:OnFailure
      (Utilities|LogError "Error marking expedition as done" _error))))

(event Custom|Watch%20Number%20of%20Players
  (params (Enable :type Boolean))
  (bind _game_ref (Variables|Default|GetGame%20Ref))
  (bind _returnvalue (Class|DatabaseReferenceProxy|Child _game_ref "players"))
  ;[1 1 1] Configure listeners for player counts
  (if Enable
    (bind _snapshot (|AddValueListener _returnvalue)
      (:OnValueChanged
        (Variables|Default|SetNumber%20of%20Players (Class|DataSnapshotProxy|ChildrenCount _snapshot))))
    (else
      (Class|QueryProxy|RemoveChildListener _returnvalue))))

(event Custom|CancelGame
  ;[1 1 1] Handle commander cancellation of a game
  (Development|PrintString "Called CancelGame")
  (Utilities|DeleteGamefromFirebase
    (:Done
      (Default|CallOnGameDeleted))))

(event Custom|Join%20Game
  (params (GameCode :type String))
  ;[1 1 1] Join Game
  (Utilities|FindandJoinGame GameCode
    (:Done
      ;[1 1 1] Manage mission abort on disconnect
      (Utilities|ConfigureAbortMissiononDisconnect
        (:Done
          (Utilities|WatchforMissionAbort
            (:Done
              (Variables|Default|SetInGame true))))))))

(event EventLoadfromGameInstance
  ;[1 1 1] Reconstruct this facade from the information in the game instance, probably because of a level change.
  (bind _asbp_collaboration_station_game_instance (Utilities|Casting|CastToBP_CollaborationStationGameInstance (Game|GetGameInstance)))
  (Utilities|FlowControl|Sequence
    (:then_0
      (Variables|Default|SetPlayerIndex (.playerindex (Variables|/Game/BP_CollaborationStationGameInstance.BP_CollaborationStationGameInstance_C|GetFacadeMemento _asbp_collaboration_station_game_instance))))
    (:then_1
      (Variables|Default|SetRoundNumber (.roundnumber (Variables|/Game/BP_CollaborationStationGameInstance.BP_CollaborationStationGameInstance_C|GetFacadeMemento _asbp_collaboration_station_game_instance))))
    (:then_2
      (Variables|Default|SetGame%20Ref (Class|RealtimeDatabaseLibrary|GetDatabaseReferencefromPath (Utilities|String|Append "games/" (.gamekey (Variables|/Game/BP_CollaborationStationGameInstance.BP_CollaborationStationGameInstance_C|GetFacadeMemento _asbp_collaboration_station_game_instance))))))
    (:then_3
      (Variables|Default|SetNumber%20of%20Players (.numberofplayers (Variables|/Game/BP_CollaborationStationGameInstance.BP_CollaborationStationGameInstance_C|GetFacadeMemento _asbp_collaboration_station_game_instance))))
    (:then_4
      (Variables|Default|SetIsCountryAssigned (.countryassigned (Variables|/Game/BP_CollaborationStationGameInstance.BP_CollaborationStationGameInstance_C|GetFacadeMemento _asbp_collaboration_station_game_instance))))
    (:then_5
      (Variables|Default|SetCountry (.country (Variables|/Game/BP_CollaborationStationGameInstance.BP_CollaborationStationGameInstance_C|GetFacadeMemento _asbp_collaboration_station_game_instance)))
      ;[1 1 1] Manage mission abort on disconnect
      (Utilities|ConfigureAbortMissiononDisconnect
        (:Done
          (Utilities|WatchforMissionAbort
            (:Done
              (Variables|Default|SetInGame true))))))))

(fn ConstructionScript)

(fn GenerateCode
  (bind _returnvalue (Game|ConstructObjectfromClass "/Script/CollaborationStation.NetworkGameIdGenerator" self))
  (return (Class|NetworkGameIdGenerator|NetworkGameIdtoString (Class|NetworkGameIdGenerator|GenerateNetworkGameId _returnvalue))))

(fn DeterminePlayerIndex
  (params (Game%20Ref :type Database%20Reference%20Proxy%20Object%20Reference) (Snapshot :type Data%20Snapshot%20Proxy%20Object%20Reference))
  (bind _returnvalue (Class|UltimateMobileKitAuth|GetLoggedUser))
  (bind _index (Utilities|FlowControl|ForLoopwithBreak 0 3 :!label _label)
    (:LoopBody
      (if (Utilities|Enum|Equal(Enum) (Class|DatabaseVariantProxy|StringValue (Class|DataSnapshotProxy|Value (Class|DataSnapshotProxy|Child Snapshot (Utilities|String|Append "players/" (Utilities|String|ToString(Integer) _index) "/uid")))) (.userid _returnvalue))
        (Variables|Default|SetPlayerIndex _index)
        (goto _label Break)))
    (:Completed
      (if (== (Variables|Default|GetPlayerIndex) -1)
        (Development|PrintString "COULD NOT FIND PLAYER INDEX")
        (else
          (Default|CallGameJoinedDispatcher true Game%20Ref)
          (return (Variables|Default|GetPlayerIndex)))))))

(fn CountPlayerswithMinigameSelection
  (params (Round :type Integer) (Snapshot :type Data%20Snapshot%20Proxy%20Object%20Reference))
  (for _index (range 0 (- (Variables|Default|GetNumber%20of%20Players) 1))
    (if (Class|DatabaseVariantProxy|IsNull (Class|DataSnapshotProxy|Value (Class|DataSnapshotProxy|Child Snapshot (Utilities|String|Append (Utilities|String|ToString(Integer) _index) "/round-" (Utilities|String|ToString(Integer) Round) "/selection"))))
      (Development|PrintString "Found a null value")
      (else
        (Development|PrintString "Found a non-null value, incrementing the thing")
        (Math|Integer|IncrementInt (LocalVariables|GetPlayersWithMinigamesSelected)))))
  (return (LocalVariables|GetPlayersWithMinigamesSelected)))

(fn IsCommander
  (return (== (Variables|Default|GetPlayerIndex) 0)))

(fn DoAllPlayersHaveScoresSet
  (params (Snapshot :type Data%20Snapshot%20Proxy%20Object%20Reference))
  (if (CallFunction|IsCommander)
    (for _index (range 0 (- (Variables|Default|GetNumber%20of%20Players) 1))
      (if (Class|DatabaseVariantProxy|IsNull (Class|DataSnapshotProxy|Value (Class|DataSnapshotProxy|Child Snapshot (Utilities|String|Append (Utilities|String|ToString(Integer) _index) "/round-" (Utilities|String|ToString(Integer) (Variables|Default|GetRoundNumber)) "/score"))))
        (return false)))
    (return true)
    (else
      (Development|PrintString "This should only be called by the commander!"))))

(fn IsFinalRound
  (bind _asbp_collaboration_station_game_instance (Utilities|Casting|CastToBP_CollaborationStationGameInstance (Game|GetGameInstance)))
  (return (== (Variables|Default|GetRoundNumber) (Utilities|Array|Length (Variables|/Script/CollaborationStation.MultiplayerGameGoals|GetPoints (Variables|/Script/CollaborationStation.CollaborationStationGameInstance|GetMultiplayerGameGoals _asbp_collaboration_station_game_instance))))))

(fn ToCountryCode
  (params (String :type String))
  (switch string String
    (:Default
      (Development|PrintString (Utilities|String|Append "Unrecognized string country code: " String))
      (return "Canada"))
    (:ca
      (return "Canada"))
    (:ch
      (return "China"))
    (:eu
      (return "EU"))
    (:ru
      (return "Russia"))
    (:us
      (return "USA"))))

(fn IsTimetoSetCountryCode
  (params (A :type String))
  (return (and (Utilities|Enum|Equal(Enum) A "brief") (not (Variables|Default|GetIsCountryAssigned)))))

(fn IncrementVariablebyInteger
  (params (Variable :type Integer%20%28by%20ref%29) (Amount :type Integer))
  (|Assign Variable (+ Variable Amount)))

(fn ShowAbortDialog
  (Development|PrintString "EXPEDITION ABORTED" false true "(R=1.000000,G=0.056108,B=0.000000,A=1.000000)" 2e+01)
  (bind _returnvalue (UserInterface|CreateWidget "/Game/UI/Widget_AbortedDialog.Widget_AbortedDialog_C" (Game|GetPlayerController 0)))
  (UserInterface|Viewport|AddtoViewport _returnvalue 0))