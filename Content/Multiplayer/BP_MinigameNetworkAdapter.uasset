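; Network adapter that links a minigame to Firebase to handle multiplayer score posting and the move to debrief.
; On BeginPlay it spawns a Firebase facade restored from the game instance and watches game state on every player.
; When the minigame is done it posts the score.
; The commander alone watches for all scores and triggers debrief, which each player relays to the game mode through the state change.
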(event Custom|OnAllPlayersPostedScores
  (bind _firebasefacade (Variables|Default|GetFirebaseFacade))
  ;[1 1 1] Commander: go to debrief when all players have a score
  (EventDispatchers|UnbindEventfromOnAllPlayersPostedScores (Variables|Default|GetFirebaseFacade) (delegate Custom|OnAllPlayersPostedScores))
  (Default|WatchPlayerScores _firebasefacade false)
  (Default|ProceedtoDebrief _firebasefacade))

(event Custom|OnGameStateChanged
  (params (New%20State :type String))
  (bind _firebasefacade (Variables|Default|GetFirebaseFacade))
  ;[1 1 1] All players watch the game state to know when to go to debrief
  (switch string New%20State
    (:debrief
      (EventDispatchers|UnbindEventfromGameStateChanged _firebasefacade (delegate Custom|OnGameStateChanged))
      (Default|WatchGameState _firebasefacade false)
      (bind _asminigame_game_mode (Utilities|Casting|CastToMinigameGameMode (Game|GetGameMode)))
      (Default|CallOnDebriefAvailable _asminigame_game_mode))))

(event EventBeginPlay
  ;[1 1 1] Reconstruct firebase facade upon starting the game
  (bind _output_get (Variables|Default|SetFirebaseFacade (CallFunction|LookupFirebaseFacade)))
  ;[1 1 1] All players watch the game state to know when to go to debrief
  (EventDispatchers|BindEventtoGameStateChanged (Variables|Default|GetFirebaseFacade) (delegate Custom|OnGameStateChanged))
  (Default|WatchGameState (Variables|Default|GetFirebaseFacade) true)
  ;[1 1 1] Commander watches for all the scores to be posted
  (if (Default|IsCommander _output_get)
    (EventDispatchers|BindEventtoOnAllPlayersPostedScores (Variables|Default|GetFirebaseFacade) (delegate Custom|OnAllPlayersPostedScores))
    (Default|WatchPlayerScores (Variables|Default|GetFirebaseFacade) true)))

(event EventOnMinigameStateChange
  (params (NewState :type EMinigameState%20Enum :default "Playing") (OldState :type EMinigameState%20Enum :default "Playing"))
  ;[1 1 1] On minigame end, write score to Firebase
  (switch Utilities|FlowControl|Switch|SwitchonEMinigameState NewState
    (:Done
      (bind _asminigame_game_mode (Utilities|Casting|CastToMinigameGameMode (Game|GetGameMode))
        (:then
          (Default|MarkRoundComplete (Variables|Default|GetFirebaseFacade) (Class|MinigameGameMode|GetScore _asminigame_game_mode)))
        (:CastFailed
          (Development|PrintString "Unexpected cast fail to minigamegamemode"))))))

(fn ConstructionScript)

(fn LookupFirebaseFacade
  (bind _returnvalue (Game|SpawnActorfromClass "/Game/Multiplayer/BP_FirebaseFacade.BP_FirebaseFacade_C" (Transformation|GetActorTransform) "Undefined" 0 0))
  (Class|NetworkFacade|LoadfromGameInstance _returnvalue)
  (return _returnvalue))