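; BP_InitialBriefingTransaction is a multiplayer database transaction that assigns each player a random country and moves the game state to "brief".
; DoTransaction builds a shuffled list from the country enum, then pops one code per entry under "players" and writes it as that player's country string.
; Popping from the shuffled list gives each player a different country.
; Null data returns success without changes.
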(fn DoTransaction
  (params (MutableData :type Mutable%20Data%20Proxy%20Object%20Reference))
  (bind _returnvalue (Class|MutableDataProxy|Child MutableData "players"))
  (if (Class|DatabaseVariantProxy|IsNull (Class|MutableDataProxy|Value MutableData))
    (return "TransactionResultSuccess")
    (else
      (bind _countrycodes (CallFunction|MakeShuffledCountryCodesArray))
      (Variables|Default|SetCountryCodes _countrycodes)
      (for _index (range 0 (- (Class|MutableDataProxy|ChildrenCount _returnvalue) 1))
        (CallFunction|AssignRandomCountryCode _returnvalue _index))
      (Class|MutableDataProxy|SetValue (Class|MutableDataProxy|Child MutableData "state") (Class|DatabaseVariantProxy|ConstructfromString "brief")))))

(fn MakeShuffledCountryCodesArray
  (bind _output_get (Variables|Default|SetCountryCodes (Utilities|Array|MakeArray)))
  (bind _enumvalue (|ForEachECountry)
    (:LoopBody
      (Utilities|Array|Add _output_get _enumvalue))
    (:then
      (Utilities|Array|Shuffle _output_get)
      (return _output_get))))

(fn Pop
  (params (CountryCodes :type Array%20of%20ECountry%20Enums :default "Canada"))
  (bind _output_get (LocalVariables|SetCode (Utilities|Array|Get(acopy) CountryCodes)))
  (Utilities|Array|RemoveIndex CountryCodes)
  (return _output_get))

(fn AssignRandomCountryCode
  (params (PlayersNode :type Mutable%20Data%20Proxy%20Object%20Reference) (PlayerIndex :type Integer))
  (bind _country (CallFunction|Pop (Variables|Default|GetCountryCodes)))
  (Class|MutableDataProxy|SetValue (Class|MutableDataProxy|Child PlayersNode (Utilities|String|Append (Utilities|String|ToString(Integer) PlayerIndex) "/country")) (Class|DatabaseVariantProxy|ConstructfromString (Utilities|ToCountryString _country))))