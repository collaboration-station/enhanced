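; BP_Jukebox is a music player that switches between main menu and task selection tracks.
; Its two events, PlayMainMenuMusic and PlayTaskSelectionMusic, each pass their track to a shared ChangeTrack function.
; ChangeTrack stops any valid CurrentlyPlaying audio, stores the new track as current and plays it from the start, with no fade.
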(event Custom|PlayMainMenuMusic
  (CallFunction|ChangeTrack (Variables|Default|GetMainMenuMusic)))

(event Custom|PlayTaskSelectionMusic
  (CallFunction|ChangeTrack (Variables|Default|GetTaskSelectionMusic)))

(fn ConstructionScript)

(fn ChangeTrack
  (params (Audio :type Audio%20Component%20Object%20Reference))
  (if (Utilities|IsValid (Variables|Default|GetCurrentlyPlaying))
    (Audio|Components|Audio|Stop (Variables|Default|GetCurrentlyPlaying)))
  (bind _output_get (Variables|Default|SetCurrentlyPlaying Audio))
  (Audio|Components|Audio|Play _output_get 0.0))