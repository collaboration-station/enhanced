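; Player controller for the menu that sets UI-only input and initializes Firebase on BeginPlay.
; Unless the game instance's NetworkStatus already indicates success, it chains two subsystem Init calls into an anonymous sign-in.
; It writes the outcome to NetworkStatus, with separate values for init failure, sign-in failure and success; only a first-Init failure is logged.
; The Init steps need no network, so real connection errors surface at sign-in.
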(event EventBeginPlay
  (Input|SetInputModeUIOnly self 0 "DoNotLock")
  (Utilities|InitializeFirebaseasNecessary))

(event EventTick
  (params (DeltaSeconds :type Float%20%28single-precision%29)))

(fn ConstructionScript)